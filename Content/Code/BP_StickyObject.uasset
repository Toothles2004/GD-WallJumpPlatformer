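; BP_StickyObject is an interactable actor that toggles between being attached to and detached from the actor that interacts with it.
; Interact checks for an attach parent: if none, it attaches to the interacting actor with keep-relative rules, calls IncreaseScale and turns green.
; If already attached, it detaches in place with keep-world rules and turns white, without a matching scale call.
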(event `/Game/Code/BI_Interactable.Interact`
  (params (otherActor :type "Actor Object Reference"))
  (if (`KismetSystemLibrary.IsValid` (`self.GetAttachParentActor`))
    (`self.K2_DetachFromActor` "KeepWorld" "KeepWorld" "KeepWorld")
    (`KismetSystemLibrary.PrintString` "detached")
    (`self.ChangeColor` (struct :`R` 1.0 :`G` 1.0 :`B` 1.0 :`A` 1.0))
    (else
      (`self.K2_AttachToActor` otherActor "None" "KeepRelative" "KeepRelative" "KeepRelative")
      (`KismetSystemLibrary.PrintString` "attached")
      (`self.IncreaseScale` 0.5 0.5)
      (`self.ChangeColor` (struct :`G` 1.0 :`B` 0.020307 :`A` 1.0)))))

(fn `UserConstructionScript`
  (`parent.UserConstructionScript`))