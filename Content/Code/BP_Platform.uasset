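; BP_Platform is a temporary platform actor that becomes solid when activated and destroys itself after a fixed lifetime.
; ChangeMaterial activates it by applying the base material and setting IsActive, which lets Tick accumulate TotalTime.
; On the first active tick the mesh starts blocking Pawns.
; Late in the countdown, chained Delays flash it between transparent and base materials as a warning before destruction.
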(event `self.ReceiveTick`
  (params (DeltaSeconds :type "Float (single-precision)"))
  (if (`self.IsActive`)
    (set `self.TotalTime` (+ DeltaSeconds (`self.TotalTime`)))
    (`|ExecutionSequence`
      (:`then_0`
        (`/Engine/EditorBlueprintResources/StandardMacros.DoOnce` false
          (:`Completed`
            (`PrimitiveComponent.SetCollisionResponseToChannel` (`self.StaticMesh`) "ECC_Pawn" "ECR_Block"))))
      (:`then_1`
        (`KismetSystemLibrary.Delay` 0.5)
        (if (>= (`self.TotalTime`) 7.5)
          (`PrimitiveComponent.SetMaterial` (`self.StaticMesh`) 0 "/Game/Data/Materials/transparent.transparent")
          (`KismetSystemLibrary.Delay` 0.2)
          (`PrimitiveComponent.SetMaterial` (`self.StaticMesh`) 0 "/Game/Data/Materials/M_BaseMaterial.M_BaseMaterial")))
      (:`then_2`
        (if (>= (`self.TotalTime`) 10.0)
          (`self.K2_DestroyActor`))))))

(fn `ChangeMaterial`
  (`PrimitiveComponent.SetMaterial` (`self.StaticMesh`) 0 "/Game/Data/Materials/M_BaseMaterial.M_BaseMaterial")
  (set `self.IsActive` true))

(fn `UserConstructionScript`)